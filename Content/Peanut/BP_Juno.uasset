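; BP_Juno is a character that idles in a looping animation and performs paired kiss and hug interactions with the player.
; Kiss snaps the player to the Vic reference transform, disables input, forces third-person camera and plays both cheek-kiss animations, then restores input and idle after a delay.
; A CanInteract toggle makes every other Kiss call only clear the flag.
; Hug plays a montage and returns Vic's location and Juno's rotation.
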(event `self.ReceiveBeginPlay`
  ;[1 1 1] Set Idle Animation on Game Start
  (`SkeletalMeshComponent.PlayAnimation` (`self.Mesh`) "/Game/ActorCore_Sample_Motions/Pose_dance_catwalk_Female/Idle_Anim.Idle_Anim" true))

(event `/Game/Peanut/BPI_Kiss.Kiss`
  (bind _returnvalue (`GameplayStatics.GetPlayerCharacter` 0))
  (bind (_returnvalue_location _returnvalue_rotation) (`KismetMathLibrary.BreakTransform` (`SceneComponent.K2_GetComponentToWorld` (`self.Vic`))))
  ;[1 1 1] Check For Overlap and Toggle Boolean For Function
  (if (not (`self.canInteract`))
    (set `self.canInteract` true)
    ;[1 1 1 1 17] Cast to Referance Cameras
    (bind _asbp_character (cast `/Game/ThirdPerson/Blueprints/BP_Character` _returnvalue))
    ;[1 1 1] Set Location/Rotation
    (`self.K2_SetActorTransform` _asbp_character (`KismetMathLibrary.MakeTransform` _returnvalue_location _returnvalue_rotation) false false)
    ;[1 1 1] Disable Inputs and Force 3rd Person Camera
    (`self.DisableInput` _returnvalue null)
    (`ActorComponent.SetActive` (`/Game/ThirdPerson/Blueprints/BP_Character.FirstPerson` _asbp_character) false false)
    (`ActorComponent.SetActive` (`/Game/ThirdPerson/Blueprints/BP_Character.ThirdPerson` _asbp_character) true false)
    ;[1 1 1] Play Animations
    (`SkeletalMeshComponent.PlayAnimation` (`Character.Mesh` _returnvalue) "/Game/Characters/Animations/Kiss/Paired_Couple_KissOnCheek01_Vic1.Paired_Couple_KissOnCheek01_Vic1" false)
    (`SkeletalMeshComponent.PlayAnimation` (`self.Mesh`) "/Game/Characters/Animations/Kiss/Paired_Couple_KissOnCheek01_Att1.Paired_Couple_KissOnCheek01_Att1" false)
    ;[1 1 1] Set Back to Default
    (`KismetSystemLibrary.Delay` 3.0)
    (`self.EnableInput` _returnvalue null)
    (`SkeletalMeshComponent.PlayAnimation` (`self.Mesh`) "/Game/ActorCore_Sample_Motions/Pose_dance_catwalk_Female/Idle_Anim.Idle_Anim" true)
    (else
      (set `self.canInteract` false))))

(fn `Hug`
  (returns (`REF Location` :type "Vector Structure") (`VIC Rotation` :type "Rotator Structure"))
  (`self.PlayAnimMontage` "/Game/Characters/Animations/Hug/Paired_Idle_Standing_Hug_Montage.Paired_Idle_Standing_Hug_Montage")
  (return (`SceneComponent.K2_GetComponentLocation` (`self.Vic`)) (`self.K2_GetActorRotation`)))

(fn `UserConstructionScript`)