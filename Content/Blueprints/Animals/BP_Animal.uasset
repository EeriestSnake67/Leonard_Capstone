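; BP_Animal is an AI-driven animal pawn that roams, makes periodic sounds and attacks the player.
; It wanders between random reachable navmesh points, pausing after each successful move, while a separate loop plays its sound at random intervals.
; When PawnSensing spots a "Player"-tagged pawn, it approaches and plays an attack montage, guarded by IsAttacking.
; A montage notify triggers a forward sphere trace that damages the hit pawn.
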(event `self.ReceiveBeginPlay`
  (`self.Wonder Around`)
  (`KismetSystemLibrary.Delay` (`KismetMathLibrary.RandomFloatInRange` 7.0 20.0) :!label _label)
  (`GameplayStatics.PlaySoundAtLocation` (`self.Animal Sound`) (`self.K2_GetActorLocation`) (struct) 0.7 1.0 0.0 "/Game/Audio/SA_Character.SA_Character" null null null)
  (goto _label))

(event `Wonder Around`
  (`|AIMoveTo` self (`NavigationSystemV1.K2_GetRandomReachablePointInRadius` (`self.K2_GetActorLocation`) 5000.0 null null) null
    (:`OnSuccess`
      (`KismetSystemLibrary.Delay` 3.0)
      (`self.Wonder Around`))))

(event `self.PawnSensing.OnSeePawn`
  (params (Pawn :type "Pawn Object Reference"))
  (bind _returnvalue (`self.K2_GetActorLocation`))
  (if (`self.ActorHasTag` Pawn "Player")
    (`|AIMoveTo` self (0.0 0.0 0.0) (`GameplayStatics.GetPlayerCharacter` 0) 400.0
      (:`OnSuccess`
        (if (not (`self.isAttacking`))
          (set `self.isAttacking` true)
          (`|PlayMontage` (`self.Mesh`) (`self.Attack Montage`)
            (:`then`
              (`GameplayStatics.PlaySoundAtLocation` (`self.Animal Sound`) (`self.K2_GetActorLocation`) (struct) 1.0 1.0 0.0 "/Game/Audio/SA_Character.SA_Character" null null null))
            (:`OnCompleted`
              (set `self.isAttacking` false))
            (:`OnNotifyBegin`
              (bind (_outhit _returnvalue_2) (`KismetSystemLibrary.SphereTraceSingleForObjects` :`Start` _returnvalue :`End` (+ _returnvalue (* (`KismetMathLibrary.GetForwardVector` (`self.K2_GetActorRotation`)) 350.0)) :`Radius` 130.0 :`ObjectTypes` (`|MakeArray` "ObjectTypeQuery3" :!type "EObjectTypeQuery Enum") :`DrawDebugType` "ForDuration"))
              (if _returnvalue_2
                (`GameplayStatics.ApplyDamage` (`.HitActor` (`GameplayStatics.BreakHitResult` _outhit)) (`self.Attack Damage`))))))))))

(fn `UserConstructionScript`)