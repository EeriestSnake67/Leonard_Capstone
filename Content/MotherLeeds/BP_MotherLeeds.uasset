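; BP_MotherLeeds is a ghost enemy that idles in a curled squat and kills the player on touch.
; On overlap with BP_Character it disables input, forces the third-person camera, snaps the player to the Victim transform and plays death and scream animations.
; After a six-second delay it reopens ThirdPersonMap.
; The construction script attaches a Hair mesh that follows the body's pose via leader pose.
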(event `self.ReceiveBeginPlay`
  ;[1 1 1] Set Idle Animation on Game Start
  (`SkeletalMeshComponent.PlayAnimation` (`self.Mesh`) "/Game/ClassicFemaleGhost/AnimSequence/UE5/ClassicFemaleGhost_Idle_CurledSquat.ClassicFemaleGhost_Idle_CurledSquat" true))

(event `self.ReceiveActorBeginOverlap`
  (params (OtherActor :type "Actor Object Reference"))
  (bind _returnvalue (`GameplayStatics.GetPlayerCharacter` 0))
  (bind (_returnvalue_location _returnvalue_rotation) (`KismetMathLibrary.BreakTransform` (`SceneComponent.K2_GetComponentToWorld` (`self.Victim`))))
  ;[1 1 1] Check For Overlap and Call Character Blueprint
  (bind _asbp_character (cast `/Game/ThirdPerson/Blueprints/BP_Character` OtherActor))
  ;[1 1 1] Disable Inputs and Force 3rd Person Camera
  (`self.DisableInput` _asbp_character null)
  (`ActorComponent.SetActive` (`/Game/ThirdPerson/Blueprints/BP_Character.FirstPerson` _asbp_character) false false)
  (`ActorComponent.SetActive` (`/Game/ThirdPerson/Blueprints/BP_Character.ThirdPerson` _asbp_character) true false)
  ;[1 1 1] Make Character Face Position
  (`self.K2_SetActorRotation` :`self` _returnvalue)
  (`self.K2_SetActorTransform` _returnvalue (`KismetMathLibrary.MakeTransform` _returnvalue_location _returnvalue_rotation) false false)
  ;[1 1 1] Play Animations
  (`SkeletalMeshComponent.PlayAnimation` (`Character.Mesh` _asbp_character) "/Game/Characters/Animations/Deaths/Death_BodyMangle03.Death_BodyMangle03" false)
  (`SkeletalMeshComponent.PlayAnimation` (`self.Mesh`) "/Game/ClassicFemaleGhost/AnimSequence/UE5/ClassicFemaleGhost_Idle_Scream01.ClassicFemaleGhost_Idle_Scream01" false)
  ;[1 1 1] Delay to Restart Level
  (`KismetSystemLibrary.Delay` 6.0)
  (`GameplayStatics.OpenLevel` "ThirdPersonMap"))

(fn `UserConstructionScript`
  (bind _hair (`self.Hair`))
  (`SkeletalMeshComponent.SetSkeletalMeshAsset` _hair "/Game/ClassicFemaleGhost/Demo/Props/Hair/SkeletalMesh_Hair.SkeletalMesh_Hair")
  (`SkinnedMeshComponent.SetLeaderPoseComponent` _hair (`self.Mesh`) false false))